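; Pong ball that moves continuously, bounces off walls and paddles, and resets on reaching a back wall.
; Tick feeds Velocity into the movement component as input.
; Sphere overlaps check actor tags: vertical walls and paddles invert X direction, horizontal walls invert Y, and back walls call ResetBall.
; Direction and reset logic are called through functions not defined in these graphs.
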(event OnComponentBeginOverlap(Sphere)
  (params (OverlappedComponent :type Primitive%20Component%20Object%20Reference) (OtherActor :type Actor%20Object%20Reference) (OtherComp :type Primitive%20Component%20Object%20Reference) (OtherBodyIndex :type Integer) (bFromSweep :type Boolean) (SweepResult :type Hit%20Result%20Structure%20%28by%20ref%29))
  (bind _returnvalue (Class|PongBall|GetCurrentDirection))
  (bind _returnvalue_2 (Class|PongBall|GetCurrentDirection))
  (if (Actor|ActorHasTag OtherActor "VerticalWall")
    (Class|PongBall|SetCurrentDirection (Math|Vector|MakeVector (* (.x _returnvalue_2) -1.0) (.y _returnvalue_2) (.z _returnvalue_2)) :!label _label)
    (elif (Actor|ActorHasTag OtherActor "Paddle")
      (goto _label)
      (elif (Actor|ActorHasTag OtherActor "HorizontalWall")
        (Class|PongBall|SetCurrentDirection (Math|Vector|MakeVector (.x _returnvalue) (* (.y _returnvalue) -1.0) (.z _returnvalue)))
        (elif (Actor|ActorHasTag OtherActor "BackWall")
          (Class|PongBall|ResetBall))))))

(event EventBeginPlay)

(event Collision|EventActorBeginOverlap
  (params (OtherActor :type Actor%20Object%20Reference)))

(event EventTick
  (params (DeltaSeconds :type Float%20%28single-precision%29))
  (Class|PawnMovementComponent|AddInputVector (Variables|Default|GetMovementComponent) (Variables|Default|GetVelocity) false))

(fn ConstructionScript)